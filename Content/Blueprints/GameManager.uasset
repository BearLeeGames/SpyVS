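; Game manager that runs a minigame loop in which the player steals code before running out of lives.
; A random looping MultiGate picks Typing, Clicking or XOR, shows its title, then spawns that widget with a manager reference.
; MinigameFinished adds remaining time to stolen code on a win or removes a life on a loss.
; MainMapUI displays progress and lives; reaching the code target or game over returns to MainMenu.
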(event EventStartMinigame
  (bind _minigame_title_delay (Variables|Default|GetMinigame%20Title%20Delay))
  (bind _main_map_ui (Variables|Default|GetMain%20Map%20UI))
  ;[1 1 1] Minigame Decider
  (Utilities|FlowControl|MultiGate true true -1
    (:Out%200
      (Class|MinigameCommunication|ShowMinigameTitle(Message) _main_map_ui "Typing")
      (Utilities|FlowControl|Delay _minigame_title_delay)
      (Class|MinigameCommunication|HideMinigameTitle(Message) _main_map_ui)
      (Utilities|StartMinigameTyping))
    (:Out%201
      (Class|MinigameCommunication|ShowMinigameTitle(Message) _main_map_ui "Clicking")
      (Utilities|FlowControl|Delay _minigame_title_delay)
      (Class|MinigameCommunication|HideMinigameTitle(Message) _main_map_ui)
      (Utilities|StartMinigameFastClick))
    (:Out%202
      (Class|MinigameCommunication|ShowMinigameTitle(Message) _main_map_ui "XOR")
      (Utilities|FlowControl|Delay _minigame_title_delay)
      (Class|MinigameCommunication|HideMinigameTitle(Message) _main_map_ui)
      (Utilities|StartMinigameXOR))))

(event EventGameOver
  ;[1 1 1] Game Over (all lives lost)
  (Utilities|FlowControl|Delay 5.0)
  (Game|OpenLevel(byName) "MainMenu"))

(event EventBeginPlay
  ;[1 1 1] Game Initialization
  (bind _returnvalue (UserInterface|CreateWidget "/Game/Blueprints/MainMapUI.MainMapUI_C"))
  (bind _output_get (Variables|Default|SetMain%20Map%20UI _returnvalue))
  (UserInterface|Viewport|AddtoViewport _output_get 10)
  (Class|MinigameCommunication|UpdateLifeCounter(Message) (Variables|Default|GetMain%20Map%20UI) (Variables|Default|GetPlayer%20Lives))
  (Class|MinigameCommunication|StartMinigame(Message) self))

(event EventMinigameFinished
  (params (Win%20State :type Boolean) (Time%20Left :type Integer))
  (bind _main_map_ui (Variables|Default|GetMain%20Map%20UI))
  (bind _main_map_ui_2 (Variables|Default|GetMain%20Map%20UI))
  ;[1 1 1] Grab Minigame Results
  (Class|MinigameCommunication|ReportMinigameCondition(Message) _main_map_ui_2 Win%20State)
  (Utilities|FlowControl|Delay 3.0)
  (Class|MinigameCommunication|HideMinigameReport(Message) _main_map_ui_2)
  (if Win%20State ; Win: Time left is added to \ncode stolen.\nLoss: Player Life lost.
    (bind _output_get (Variables|Default|SetStolen%20Code%20Amount (+ (Variables|Default|GetStolen%20Code%20Amount) Time%20Left)))
    (Class|MinigameCommunication|ReportProgress(Message) _main_map_ui _output_get)
    (if (>= (Variables|Default|GetStolen%20Code%20Amount) 100)
      (Class|MinigameCommunication|GameWin(Message) (Variables|Default|GetMain%20Map%20UI))
      (Utilities|FlowControl|Delay 1e+01)
      (Game|OpenLevel(byName) "MainMenu")
      (else
        (Utilities|FlowControl|Delay 2.0 :!label _label)
        (Class|MinigameCommunication|StartMinigame(Message) self)))
    (else
      (bind _result (Math|Integer|DecrementInt (Variables|Default|GetPlayer%20Lives))
        (:%20%20
          (bind _output_get_2 (Variables|Default|SetPlayer%20Lives _result))
          (Class|MinigameCommunication|UpdateLifeCounter(Message) _main_map_ui _output_get_2)
          (if (!= _output_get_2 0)
            (goto _label)
            (else
              (Class|MinigameCommunication|GameOver(Message) self))))))))

(fn ConstructionScript)