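; XORGameMode is a game mode that sets up a binary XOR puzzle when play begins.
; BeginPlay fills two arrays with random bits, joins each into a string, and stores their bitwise XOR in an Answer array.
; It then creates the XOR_HUD widget, passes it both strings as text, and adds it to the viewport.
; The answer is not sent to the HUD here, and Tick does nothing.
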(event EventBeginPlay
  (bind _returnvalue (Math|Random|RandomIntegerinRange 0 1))
  (bind _value1 (Variables|Default|GetValue1))
  ;[1 1 1] Create Value1 Array
  (for _index (range 0 5)
    (Utilities|Array|Add (Variables|Default|GetValue1) _returnvalue)
    (Utilities|Array|Add (Variables|Default|GetValue2) _returnvalue))
  ;[1 1 1] Change Int Array To String
  (for _array_element (Variables|Default|GetValue1)
    (Variables|Default|SetValue1_String (Utilities|String|Append (Variables|Default|GetValue1_String) (Utilities|String|ToString(Integer) _array_element))))
  (for _array_element_2 (Variables|Default|GetValue2)
    (Variables|Default|SetValue2_String (Utilities|String|Append (Variables|Default|GetValue2_String) (Utilities|String|ToString(Integer) _array_element_2))))
  ;[1 1 1] Get XOR Answer
  (for _index_2 (range 0 (- (Utilities|Array|Length _value1) 1))
    (Utilities|Array|Add (Variables|Default|GetAnswer) (Math|Conversions|ToInteger(Boolean) (Class|KismetMathLibrary|XORBoolean (Math|Conversions|ToBoolean(Integer) (Utilities|Array|Get(acopy) _value1 _index_2)) (Math|Conversions|ToBoolean(Integer) (Utilities|Array|Get(acopy) (Variables|Default|GetValue2) _index_2))))))
  ;[1 1 1] Set Up UI
  (bind _returnvalue_2 (UserInterface|CreateWidget "/Game/UI/XOR_HUD.XOR_HUD_C"))
  (Variables|/Game/UI/XOR_HUD.XOR_HUD_C|SetValue1Temp _returnvalue_2 (Utilities|Text|ToText(String) (Variables|Default|GetValue1_String)))
  (Variables|/Game/UI/XOR_HUD.XOR_HUD_C|SetValue2Temp _returnvalue_2 (Utilities|Text|ToText(String) (Variables|Default|GetValue2_String)))
  (UserInterface|Viewport|AddtoViewport _returnvalue_2 0))

(event EventTick
  (params (DeltaSeconds :type Float%20%28single-precision%29)))

(fn ConstructionScript)